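; Radio trigger actor that delivers one of three random breaking-news endings and closes out the level.
; On BeginPlay it hides all referenced newspaper actors, picks a random index and reveals the matching one.
; When the first-person character enters its box, it plays that index's news broadcast and removes the trigger.
; After timed delays it plays a dying beep, shows the final widget, then a loading screen and opens the menu level.
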(event OnComponentBeginOverlap(Box)
  (params (OverlappedComponent :type Primitive%20Component%20Object%20Reference) (OtherActor :type Actor%20Object%20Reference) (OtherComp :type Primitive%20Component%20Object%20Reference) (OtherBodyIndex :type Integer) (bFromSweep :type Boolean) (SweepResult :type Hit%20Result%20Structure%20%28by%20ref%29))
  (Utilities|Casting|CastToFirstPersonCharacter OtherActor)
  (switch int (Variables|Default|GetRand)
    (:0
      (Audio|PlaySound2D "/Game/Sound/VoiceOver/Breaking_News_Suicide.Breaking_News_Suicide" 1.0 1.0 0.0 0 0))
    (:1
      (Audio|PlaySound2D "/Game/Sound/VoiceOver/breakingNews_Beaten.breakingNews_Beaten" 1.0 1.0 0.0 0 0))
    (:2
      (Audio|PlaySound2D "/Game/Sound/VoiceOver/Breaking_News_Massacre.Breaking_News_Massacre" 1.0 1.0 0.0 0 0)))
  (Components|DestroyComponent (Variables|Default|GetBox))
  (Utilities|FlowControl|Delay 32.0)
  (Audio|PlaySound2D "/Game/Sound/SoundFX/DyingBeep.DyingBeep" 1.0 1.0 0.0 0 0)
  (bind _returnvalue (UserInterface|CreateWidget "/Game/FirstPersonBP/Blueprints/FinalWidget.FinalWidget_C"))
  (UserInterface|Viewport|AddtoViewport _returnvalue 1)
  (Utilities|FlowControl|Delay 6.0)
  (bind _asloading (Utilities|Casting|CastToLoading (Game|GetGameInstance)))
  (Default|ShowLoadingScreen _asloading)
  (Utilities|FlowControl|Delay 0.5)
  (Game|OpenLevel(byName) "menu"))

(event EventBeginPlay
  (for _array_element (Variables|Default|GetNewsPaper)
    (Rendering|SetActorHiddenInGame _array_element true))
  (switch int (Math|Random|RandomInteger 3)
    (:0
      (Variables|Default|SetRand 0))
    (:1
      (Variables|Default|SetRand 1))
    (:2
      (Variables|Default|SetRand 2)))
  (Rendering|SetActorHiddenInGame (Utilities|Array|Get(acopy) (Variables|Default|GetNewsPaper) (Variables|Default|GetRand)) false))

(event Collision|EventActorBeginOverlap
  (params (OtherActor :type Actor%20Object%20Reference)))

(event EventTick
  (params (DeltaSeconds :type Float%20%28single-precision%29)))

(fn ConstructionScript)